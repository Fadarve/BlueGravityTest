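; BP_SkatePlayerState is the player state for the skating game, tracking the current score and reporting made tricks.
; TrickMade adds the trick's score through AddToScore, then passes the trick to UpdateHUD, which calls DisplayMadeTrickName on the BP_SkatePC HUD.
; AddToScore also calls UpdateHUD with no trick supplied, and GetCurrentScore exposes the running total.
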(event `AddToScore`
  (params (ScoreToAdd :type Integer))
  (set `self.CurrentScore` (+ (`self.CurrentScore`) ScoreToAdd))
  (`self.UpdateHUD` (struct)))

(event `/Game/Skating/Blueprints/Game/BI_Status.TrickMade`
  (params (Trick :type "/Game/Skating/Blueprints/Obstacles/E_Trick Structure"))
  (`self.AddToScore` (`.Score_5_68E6DFB14866C15E2AD598B5C5B7C817` (break `/Game/Skating/Blueprints/Obstacles/E_Trick` Trick)))
  (`self.UpdateHUD` Trick))

(event `UpdateHUD`
  (params (TrickName :type "/Game/Skating/Blueprints/Obstacles/E_Trick Structure"))
  (bind _asbp_skate_pc (cast `/Game/Skating/Blueprints/Game/BP_SkatePC` (`self.GetPlayerController`)))
  (`/Game/Skating/Blueprints/UI/WB_PlayerHUD.DisplayMadeTrickName` (`/Game/Skating/Blueprints/Game/BP_SkatePC.HUD` _asbp_skate_pc) TrickName))

(fn `GetCurrentScore`
  (returns (Score :type Integer))
  (return (`self.CurrentScore`)))

(fn `UserConstructionScript`)