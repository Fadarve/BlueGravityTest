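; Base skating obstacle that detects when an actor jumps over it between two trigger points, in either direction.
; Leaving a point while the actor reports falling flags that point and starts a time-limit timer.
; Leaving the opposite point while flagged cancels the timer and counts a success, without rechecking falling; expiry clears the flag.
; Success leaves flags set, and outcomes only print debug messages.
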(event `self.JumpPoint1.OnComponentEndOverlap`
  (params (OverlappedComponent :type "PrimitiveComponent Object Reference") (OtherActor :type "Actor Object Reference") (OtherComp :type "PrimitiveComponent Object Reference") (OtherBodyIndex :type Integer))
  (`self.TryJump` true OtherActor))

(event `self.JumpPoint2.OnComponentEndOverlap`
  (params (OverlappedComponent :type "PrimitiveComponent Object Reference") (OtherActor :type "Actor Object Reference") (OtherComp :type "PrimitiveComponent Object Reference") (OtherBodyIndex :type Integer))
  (`self.TryJump` false OtherActor))

(event `TryJump`
  (params (IsPoint1 :type Boolean) (Actor :type "Actor Object Reference"))
  ;[1 1 1 1 35] Jump Logic
  (if (select `bool` IsPoint1 :`false` (`self.Point1Passed`) :`true` (`self.Point2Passed`))
    (`KismetSystemLibrary.K2_ClearAndInvalidateTimerHandle` (`self.JumpTimerHandle`))
    (`self.JumpSucces`)
    (else
      (bind _returnvalue (message `SkaterInterface.GetIsFalling` Actor))
      (if _returnvalue
        (if IsPoint1
          (set `self.Point1Passed` true)
          (else
            (set `self.Point2Passed` true)))
        (bind _returnvalue_2 (`KismetSystemLibrary.K2_SetTimerDelegate` (delegate `JumpFailed`) (`self.JumpTimeLimit`)))
        (set `self.JumpTimerHandle` _returnvalue_2)
        (`KismetSystemLibrary.PrintString` "Jump time limit started" true true (struct :`R` 0.325916 :`G` 0.144696 :`B` 1.0 :`A` 1.0) 3.0)))))

(event `JumpSucces`
  (`KismetSystemLibrary.PrintString` "Jumped obstacke succesfully" true true (struct :`G` 1.0 :`B` 0.114498 :`A` 1.0) 5.0))

(event `JumpFailed`
  ;[1 1 1 1 35] Jump Logic
  (if (stale `TryJump` IsPoint1)
    (set `self.Point1Passed` false)
    (else
      (set `self.Point2Passed` false)))
  (`KismetSystemLibrary.PrintString` "Jump time limit finished" true true (struct :`R` 1.0 :`A` 1.0) 3.0))

(fn `UserConstructionScript`)